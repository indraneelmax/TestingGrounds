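; AI controller for guard NPCs that runs the Guard_BT behavior tree on the Patrol blackboard.
; Perception updates store sensed actors without the IAmAEnemy tag in the blackboard's enemy key, clear it when sensing is lost, and print debug info.
; Each tick sets the controlled PatrolGuard2's Aiming flag from whether a focus actor exists.
; FindPatrolPath is an empty stub.
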(event OnTargetPerceptionUpdated(AIPerception)
  (params (Actor :type Actor%20Object%20Reference) (Stimulus :type AI%20Stimulus%20Structure))
  (bind _myblackboardcomponent (Variables|Default|GetMyBlackBoardComponent))
  (bind _enemykey (Variables|Default|GetEnemyKey))
  (Utilities|FlowControl|Sequence
    (:then_0
      ;[1 1 1] Make AI look at Player
      (if (not (Actor|ActorHasTag Actor "IAmAEnemy"))
        (if (.bSuccessfullySensed (Utilities|Struct|BreakAIStimulus Stimulus))
          (AI|Components|Blackboard|SetValueasObject _myblackboardcomponent _enemykey Actor)
          (else
            (AI|Components|Blackboard|ClearValue _myblackboardcomponent _enemykey)))))
    (:then_1
      ;[1 1 1] Printing Perception!
      (bind _returnvalue (Class|AIPerceptionSystem|GetSenseClassforStimulus Stimulus))
      (Development|PrintString (Utilities|String|Append (Utilities|GetObjectName (Pawn|GetControlledPawn)) " " (Utilities|GetClassDisplayName _returnvalue) " " (Utilities|GetObjectName Actor))))))

(event EventBeginPlay
  (bind _blackboardcomponent (Class|AIController|UseBlackboard "/Game/Dynamic/NPC/AI/Patrol.Patrol"))
  (AI|RunBehaviorTree "/Game/Dynamic/NPC/AI/Guard_BT.Guard_BT")
  (Variables|Default|SetMyBlackBoardComponent _blackboardcomponent))

(event EventTick
  (params (DeltaSeconds :type Float%20%28single-precision%29))
  ;[1 1 1] Set aiming/focus when detect an actor
  (bind _aspatrol_guard_2 (Utilities|Casting|CastToPatrolGuard2 (Pawn|GetControlledPawn)))
  (Variables|/Game/Dynamic/NPC/Behaviour/PatrolGuard2.PatrolGuard2_C|SetAiming _aspatrol_guard_2 (Utilities|IsValid (Class|AIController|GetFocusActor))))

(fn ConstructionScript)

(fn FindPatrolPath
  (params (BlackBoard :type Blackboard%20Component%20Object%20Reference)))